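; BP_ChessPawn is a chess piece pawn that fights, with health, a team color and an overhead HP widget.
; On BeginPlay it initializes the BP_HP widget, which turns toward the camera every tick, and incoming damage lowers health until the pawn is destroyed.
; DoAttack cycles through the attack montages, DoDamage damages the current target, and SetTeam tints the skeletal mesh's BodyColor red or green.
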(event `self.ReceiveBeginPlay`
  (bind _asbp_hp (cast `/Game/Blueprint/UI/BP_HP` (`WidgetComponent.GetUserWidgetObject` (`self.Widget`))))
  (`/Game/Blueprint/UI/BP_HP.InitUI` _asbp_hp self))

(event `self.ReceiveTick`
  (params (DeltaSeconds :type "Float (single-precision)"))
  (bind _widget (`self.Widget`))
  (`SceneComponent.K2_SetWorldRotation` _widget (`KismetMathLibrary.FindLookAtRotation` (`SceneComponent.K2_GetComponentLocation` _widget) (`self.K2_GetActorLocation` (`GameplayStatics.GetPlayerCameraManager` 0))) false false))

(event `self.ReceiveAnyDamage`
  (params (Damage :type "Float (single-precision)") (DamageType :type "DamageType Object Reference") (InstigatedBy :type "Controller Object Reference") (DamageCauser :type "Actor Object Reference"))
  (bind _output_get (set `self.Health` (`KismetMathLibrary.FMax` (- (`self.Health`) Damage))))
  (if (<= _output_get 0.0)
    (`self.K2_DestroyActor`)))

(fn `DoAttack`
  (returns (Return :type "Float (double-precision)"))
  (bind _attackmontages (`self.AttackMontages`))
  (bind _attackmontagelndex (`self.AttackMontagelndex`))
  (if (`KismetArrayLibrary.Array_IsValidIndex` _attackmontages)
    (if (> _attackmontagelndex (- (`KismetArrayLibrary.Array_Length` _attackmontages) 1))
      (set `self.AttackMontagelndex` 0))
    (bind _returnvalue (`AnimInstance.Montage_Play` (`SkeletalMeshComponent.GetAnimInstance` (`self.SkeletalMesh`)) (`|GetArrayItem` _attackmontages _attackmontagelndex) 1.0 "MontageLength" 0.0 true))
    (`/Engine/EditorBlueprintResources/StandardMacros.IncrementInt` (`self.AttackMontagelndex`)
      (:`  `
        (return _returnvalue)))
    (else
      (return 0.0))))

(fn `DoDamage`
  (`GameplayStatics.ApplyDamage` (`self.NowTarget`) 1.0))

(fn `SetTeam`
  (params (TeamIndex :type Integer))
  (bind _skeletalmesh (`self.SkeletalMesh`))
  (bind _output_get (set `self.TeamIndex` TeamIndex))
  (switch `int` _output_get
    (:`0`
      (`MeshComponent.SetVectorParameterValueOnMaterials` _skeletalmesh "BodyColor" (`KismetMathLibrary.Conv_LinearColorToVector` (struct :`R` 1.0 :`A` 1.0))))
    (:`1`
      (`MeshComponent.SetVectorParameterValueOnMaterials` _skeletalmesh "BodyColor" (`KismetMathLibrary.Conv_LinearColorToVector` (struct :`G` 1.0 :`A` 1.0))))))

(fn `UserConstructionScript`)