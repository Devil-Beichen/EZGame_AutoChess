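; Grid map actor for a chess-style game that spawns both teams' starting sword pawns on opposite edge rows of the board.
; After a short BeginPlay delay, it runs two hand-unrolled spawn macros, one per team, each filling a ten-node row.
; Each BP_ChessPawn_Sword spawns at its GetNode location, then registers that node with its ChessMovement component and receives its team index.
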(event `self.ReceiveBeginPlay`
  (bind _returnvalue (`self.GetNode` (make `GridVector` 2)))
  (bind _returnvalue_2 (`self.GetNode` (make `GridVector` 9)))
  (bind _returnvalue_3 (`self.GetNode` (make `GridVector` 5)))
  (bind _returnvalue_4 (`self.GetNode` (make `GridVector` 0)))
  (bind _returnvalue_5 (`self.GetNode` (make `GridVector` 6)))
  (bind _returnvalue_6 (`self.GetNode` (make `GridVector` 1)))
  (bind _returnvalue_7 (`self.GetNode` (make `GridVector` 7)))
  (bind _returnvalue_8 (`self.GetNode` (make `GridVector` 8)))
  (bind _returnvalue_9 (`self.GetNode` (make `GridVector` 3)))
  (bind _returnvalue_10 (`self.GetNode` (make `GridVector` 4)))
  (bind _returnvalue_11 (`self.GetNode` (make `GridVector` 7 11)))
  (bind _returnvalue_12 (`self.GetNode` (make `GridVector` 8 11)))
  (bind _returnvalue_13 (`self.GetNode` (make `GridVector` 5 11)))
  (bind _returnvalue_14 (`self.GetNode` (make `GridVector` 0 11)))
  (bind _returnvalue_15 (`self.GetNode` (make `GridVector` 4 11)))
  (bind _returnvalue_16 (`self.GetNode` (make `GridVector` 3 11)))
  (bind _returnvalue_17 (`self.GetNode` (make `GridVector` 2 11)))
  (bind _returnvalue_18 (`self.GetNode` (make `GridVector` 1 11)))
  (bind _returnvalue_19 (`self.GetNode` (make `GridVector` 9 11)))
  (bind _returnvalue_20 (`self.GetNode` (make `GridVector` 6 11)))
  (`KismetSystemLibrary.Delay` 0.2)
  (`|ExecutionSequence`
    (:`then_0`
      (`|ExecutionSequence`
        (:`then_0`
          (bind _returnvalue_21 (`|SpawnActorFromClass` "/Game/Blueprint/BP_ChessPawn_Sword.BP_ChessPawn_Sword_C" (`KismetMathLibrary.MakeTransform` (`GridNode.Location` _returnvalue_4)) "AlwaysSpawn" "OverrideRootScale" null null))
          (`/Engine/EditorBlueprintResources/StandardMacros.IsValid` _returnvalue_21
            (:`Is Valid`
              (`ChessMovementComponent.SetNowNode` (`/Game/Blueprint/BP_ChessPawn.ChessMovement` _returnvalue_21) _returnvalue_4)
              (`/Game/Blueprint/BP_ChessPawn.SetTeam` _returnvalue_21 1))))
        (:`then_1`
          (bind _returnvalue_22 (`|SpawnActorFromClass` "/Game/Blueprint/BP_ChessPawn_Sword.BP_ChessPawn_Sword_C" (`KismetMathLibrary.MakeTransform` (`GridNode.Location` _returnvalue_6)) "AlwaysSpawn" "OverrideRootScale" null null))
          (`/Engine/EditorBlueprintResources/StandardMacros.IsValid` _returnvalue_22
            (:`Is Valid`
              (`ChessMovementComponent.SetNowNode` (`/Game/Blueprint/BP_ChessPawn.ChessMovement` _returnvalue_22) _returnvalue_6)
              (`/Game/Blueprint/BP_ChessPawn.SetTeam` _returnvalue_22 1))))
        (:`then_2`
          (bind _returnvalue_23 (`|SpawnActorFromClass` "/Game/Blueprint/BP_ChessPawn_Sword.BP_ChessPawn_Sword_C" (`KismetMathLibrary.MakeTransform` (`GridNode.Location` _returnvalue)) "AlwaysSpawn" "OverrideRootScale" null null))
          (`/Engine/EditorBlueprintResources/StandardMacros.IsValid` _returnvalue_23
            (:`Is Valid`
              (`ChessMovementComponent.SetNowNode` (`/Game/Blueprint/BP_ChessPawn.ChessMovement` _returnvalue_23) _returnvalue)
              (`/Game/Blueprint/BP_ChessPawn.SetTeam` _returnvalue_23 1))))
        (:`then_3`
          (bind _returnvalue_24 (`|SpawnActorFromClass` "/Game/Blueprint/BP_ChessPawn_Sword.BP_ChessPawn_Sword_C" (`KismetMathLibrary.MakeTransform` (`GridNode.Location` _returnvalue_9)) "AlwaysSpawn" "OverrideRootScale" null null))
          (`/Engine/EditorBlueprintResources/StandardMacros.IsValid` _returnvalue_24
            (:`Is Valid`
              (`ChessMovementComponent.SetNowNode` (`/Game/Blueprint/BP_ChessPawn.ChessMovement` _returnvalue_24) _returnvalue_9)
              (`/Game/Blueprint/BP_ChessPawn.SetTeam` _returnvalue_24 1))))
        (:`then_4`
          (bind _returnvalue_25 (`|SpawnActorFromClass` "/Game/Blueprint/BP_ChessPawn_Sword.BP_ChessPawn_Sword_C" (`KismetMathLibrary.MakeTransform` (`GridNode.Location` _returnvalue_10)) "AlwaysSpawn" "OverrideRootScale" null null))
          (`/Engine/EditorBlueprintResources/StandardMacros.IsValid` _returnvalue_25
            (:`Is Valid`
              (`ChessMovementComponent.SetNowNode` (`/Game/Blueprint/BP_ChessPawn.ChessMovement` _returnvalue_25) _returnvalue_10)
              (`/Game/Blueprint/BP_ChessPawn.SetTeam` _returnvalue_25 1))))
        (:`then_5`
          (bind _returnvalue_26 (`|SpawnActorFromClass` "/Game/Blueprint/BP_ChessPawn_Sword.BP_ChessPawn_Sword_C" (`KismetMathLibrary.MakeTransform` (`GridNode.Location` _returnvalue_3)) "AlwaysSpawn" "OverrideRootScale" null null))
          (`/Engine/EditorBlueprintResources/StandardMacros.IsValid` _returnvalue_26
            (:`Is Valid`
              (`ChessMovementComponent.SetNowNode` (`/Game/Blueprint/BP_ChessPawn.ChessMovement` _returnvalue_26) _returnvalue_3)
              (`/Game/Blueprint/BP_ChessPawn.SetTeam` _returnvalue_26 1))))
        (:`then_6`
          (bind _returnvalue_27 (`|SpawnActorFromClass` "/Game/Blueprint/BP_ChessPawn_Sword.BP_ChessPawn_Sword_C" (`KismetMathLibrary.MakeTransform` (`GridNode.Location` _returnvalue_5)) "AlwaysSpawn" "OverrideRootScale" null null))
          (`/Engine/EditorBlueprintResources/StandardMacros.IsValid` _returnvalue_27
            (:`Is Valid`
              (`ChessMovementComponent.SetNowNode` (`/Game/Blueprint/BP_ChessPawn.ChessMovement` _returnvalue_27) _returnvalue_5)
              (`/Game/Blueprint/BP_ChessPawn.SetTeam` _returnvalue_27 1))))
        (:`then_7`
          (bind _returnvalue_28 (`|SpawnActorFromClass` "/Game/Blueprint/BP_ChessPawn_Sword.BP_ChessPawn_Sword_C" (`KismetMathLibrary.MakeTransform` (`GridNode.Location` _returnvalue_7)) "AlwaysSpawn" "OverrideRootScale" null null))
          (`/Engine/EditorBlueprintResources/StandardMacros.IsValid` _returnvalue_28
            (:`Is Valid`
              (`ChessMovementComponent.SetNowNode` (`/Game/Blueprint/BP_ChessPawn.ChessMovement` _returnvalue_28) _returnvalue_7)
              (`/Game/Blueprint/BP_ChessPawn.SetTeam` _returnvalue_28 1))))
        (:`then_8`
          (bind _returnvalue_29 (`|SpawnActorFromClass` "/Game/Blueprint/BP_ChessPawn_Sword.BP_ChessPawn_Sword_C" (`KismetMathLibrary.MakeTransform` (`GridNode.Location` _returnvalue_8)) "AlwaysSpawn" "OverrideRootScale" null null))
          (`/Engine/EditorBlueprintResources/StandardMacros.IsValid` _returnvalue_29
            (:`Is Valid`
              (`ChessMovementComponent.SetNowNode` (`/Game/Blueprint/BP_ChessPawn.ChessMovement` _returnvalue_29) _returnvalue_8)
              (`/Game/Blueprint/BP_ChessPawn.SetTeam` _returnvalue_29 1))))
        (:`then_9`
          (bind _returnvalue_30 (`|SpawnActorFromClass` "/Game/Blueprint/BP_ChessPawn_Sword.BP_ChessPawn_Sword_C" (`KismetMathLibrary.MakeTransform` (`GridNode.Location` _returnvalue_2)) "AlwaysSpawn" "OverrideRootScale" null null))
          (`/Engine/EditorBlueprintResources/StandardMacros.IsValid` _returnvalue_30
            (:`Is Valid`
              (`ChessMovementComponent.SetNowNode` (`/Game/Blueprint/BP_ChessPawn.ChessMovement` _returnvalue_30) _returnvalue_2)
              (`/Game/Blueprint/BP_ChessPawn.SetTeam` _returnvalue_30 1))))))
    (:`then_1`
      (`|ExecutionSequence`
        (:`then_0`
          (bind _returnvalue_31 (`|SpawnActorFromClass` "/Game/Blueprint/BP_ChessPawn_Sword.BP_ChessPawn_Sword_C" (`KismetMathLibrary.MakeTransform` (`GridNode.Location` _returnvalue_19)) "AlwaysSpawn" "OverrideRootScale" null null))
          (`/Engine/EditorBlueprintResources/StandardMacros.IsValid` _returnvalue_31
            (:`Is Valid`
              (`ChessMovementComponent.SetNowNode` (`/Game/Blueprint/BP_ChessPawn.ChessMovement` _returnvalue_31) _returnvalue_19)
              (`/Game/Blueprint/BP_ChessPawn.SetTeam` _returnvalue_31 0))))
        (:`then_1`
          (bind _returnvalue_32 (`|SpawnActorFromClass` "/Game/Blueprint/BP_ChessPawn_Sword.BP_ChessPawn_Sword_C" (`KismetMathLibrary.MakeTransform` (`GridNode.Location` _returnvalue_12)) "AlwaysSpawn" "OverrideRootScale" null null))
          (`/Engine/EditorBlueprintResources/StandardMacros.IsValid` _returnvalue_32
            (:`Is Valid`
              (`ChessMovementComponent.SetNowNode` (`/Game/Blueprint/BP_ChessPawn.ChessMovement` _returnvalue_32) _returnvalue_12)
              (`/Game/Blueprint/BP_ChessPawn.SetTeam` _returnvalue_32 0))))
        (:`then_2`
          (bind _returnvalue_33 (`|SpawnActorFromClass` "/Game/Blueprint/BP_ChessPawn_Sword.BP_ChessPawn_Sword_C" (`KismetMathLibrary.MakeTransform` (`GridNode.Location` _returnvalue_11)) "AlwaysSpawn" "OverrideRootScale" null null))
          (`/Engine/EditorBlueprintResources/StandardMacros.IsValid` _returnvalue_33
            (:`Is Valid`
              (`ChessMovementComponent.SetNowNode` (`/Game/Blueprint/BP_ChessPawn.ChessMovement` _returnvalue_33) _returnvalue_11)
              (`/Game/Blueprint/BP_ChessPawn.SetTeam` _returnvalue_33 0))))
        (:`then_3`
          (bind _returnvalue_34 (`|SpawnActorFromClass` "/Game/Blueprint/BP_ChessPawn_Sword.BP_ChessPawn_Sword_C" (`KismetMathLibrary.MakeTransform` (`GridNode.Location` _returnvalue_20)) "AlwaysSpawn" "OverrideRootScale" null null))
          (`/Engine/EditorBlueprintResources/StandardMacros.IsValid` _returnvalue_34
            (:`Is Valid`
              (`ChessMovementComponent.SetNowNode` (`/Game/Blueprint/BP_ChessPawn.ChessMovement` _returnvalue_34) _returnvalue_20)
              (`/Game/Blueprint/BP_ChessPawn.SetTeam` _returnvalue_34 0))))
        (:`then_4`
          (bind _returnvalue_35 (`|SpawnActorFromClass` "/Game/Blueprint/BP_ChessPawn_Sword.BP_ChessPawn_Sword_C" (`KismetMathLibrary.MakeTransform` (`GridNode.Location` _returnvalue_13)) "AlwaysSpawn" "OverrideRootScale" null null))
          (`/Engine/EditorBlueprintResources/StandardMacros.IsValid` _returnvalue_35
            (:`Is Valid`
              (`ChessMovementComponent.SetNowNode` (`/Game/Blueprint/BP_ChessPawn.ChessMovement` _returnvalue_35) _returnvalue_13)
              (`/Game/Blueprint/BP_ChessPawn.SetTeam` _returnvalue_35 0))))
        (:`then_5`
          (bind _returnvalue_36 (`|SpawnActorFromClass` "/Game/Blueprint/BP_ChessPawn_Sword.BP_ChessPawn_Sword_C" (`KismetMathLibrary.MakeTransform` (`GridNode.Location` _returnvalue_15)) "AlwaysSpawn" "OverrideRootScale" null null))
          (`/Engine/EditorBlueprintResources/StandardMacros.IsValid` _returnvalue_36
            (:`Is Valid`
              (`ChessMovementComponent.SetNowNode` (`/Game/Blueprint/BP_ChessPawn.ChessMovement` _returnvalue_36) _returnvalue_15)
              (`/Game/Blueprint/BP_ChessPawn.SetTeam` _returnvalue_36 0))))
        (:`then_6`
          (bind _returnvalue_37 (`|SpawnActorFromClass` "/Game/Blueprint/BP_ChessPawn_Sword.BP_ChessPawn_Sword_C" (`KismetMathLibrary.MakeTransform` (`GridNode.Location` _returnvalue_16)) "AlwaysSpawn" "OverrideRootScale" null null))
          (`/Engine/EditorBlueprintResources/StandardMacros.IsValid` _returnvalue_37
            (:`Is Valid`
              (`ChessMovementComponent.SetNowNode` (`/Game/Blueprint/BP_ChessPawn.ChessMovement` _returnvalue_37) _returnvalue_16)
              (`/Game/Blueprint/BP_ChessPawn.SetTeam` _returnvalue_37 0))))
        (:`then_7`
          (bind _returnvalue_38 (`|SpawnActorFromClass` "/Game/Blueprint/BP_ChessPawn_Sword.BP_ChessPawn_Sword_C" (`KismetMathLibrary.MakeTransform` (`GridNode.Location` _returnvalue_17)) "AlwaysSpawn" "OverrideRootScale" null null))
          (`/Engine/EditorBlueprintResources/StandardMacros.IsValid` _returnvalue_38
            (:`Is Valid`
              (`ChessMovementComponent.SetNowNode` (`/Game/Blueprint/BP_ChessPawn.ChessMovement` _returnvalue_38) _returnvalue_17)
              (`/Game/Blueprint/BP_ChessPawn.SetTeam` _returnvalue_38 0))))
        (:`then_8`
          (bind _returnvalue_39 (`|SpawnActorFromClass` "/Game/Blueprint/BP_ChessPawn_Sword.BP_ChessPawn_Sword_C" (`KismetMathLibrary.MakeTransform` (`GridNode.Location` _returnvalue_18)) "AlwaysSpawn" "OverrideRootScale" null null))
          (`/Engine/EditorBlueprintResources/StandardMacros.IsValid` _returnvalue_39
            (:`Is Valid`
              (`ChessMovementComponent.SetNowNode` (`/Game/Blueprint/BP_ChessPawn.ChessMovement` _returnvalue_39) _returnvalue_18)
              (`/Game/Blueprint/BP_ChessPawn.SetTeam` _returnvalue_39 0))))
        (:`then_9`
          (bind _returnvalue_40 (`|SpawnActorFromClass` "/Game/Blueprint/BP_ChessPawn_Sword.BP_ChessPawn_Sword_C" (`KismetMathLibrary.MakeTransform` (`GridNode.Location` _returnvalue_14)) "AlwaysSpawn" "OverrideRootScale" null null))
          (`/Engine/EditorBlueprintResources/StandardMacros.IsValid` _returnvalue_40
            (:`Is Valid`
              (`ChessMovementComponent.SetNowNode` (`/Game/Blueprint/BP_ChessPawn.ChessMovement` _returnvalue_40) _returnvalue_14)
              (`/Game/Blueprint/BP_ChessPawn.SetTeam` _returnvalue_40 0))))))))

(fn `UserConstructionScript`)